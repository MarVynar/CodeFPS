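; BP_Artefact is an environment actor that animates two small mesh components in a recurring rotation.
; BeginPlay starts a looping seven-second timer with a negative start delay to cancel the first wait, apparently driving MotionLoop.
; MotionLoop restarts a timeline whose Rot value is added to current rotation every update, pitching one mesh and yawing the other.
; Timeline completion calls OnFinishRotation, which is empty here.
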(event `self.ReceiveBeginPlay`
  (`parent.ReceiveBeginPlay`)
  (`KismetSystemLibrary.K2_SetTimerDelegate` (`|CreateDelegate` :!event `MotionLoop`) 7.0 true -7.0))

(event `MotionLoop`
  (bind _sm_monu3_small (`self.SM_Monu3_Small`))
  (bind _sm_monu3_small1 (`self.SM_Monu3_Small1`))
  (bind (_relativerotation_roll _relativerotation_pitch _relativerotation_yaw) (`KismetMathLibrary.BreakRotator` (`SceneComponent.RelativeRotation` _sm_monu3_small1)))
  (bind (_relativerotation_roll_2 _relativerotation_pitch_2) (`KismetMathLibrary.BreakRotator` (`SceneComponent.RelativeRotation` _sm_monu3_small)))
  (bind (_direction _rot) (`Timeline|Timeline_0` :!via `PlayFromStart`)
    (:`Update`
      (`SceneComponent.K2_SetRelativeRotation` _sm_monu3_small (`KismetMathLibrary.MakeRotator` 0.0 (+ _rot _relativerotation_pitch_2)) false false)
      (`SceneComponent.K2_SetRelativeRotation` _sm_monu3_small1 (`KismetMathLibrary.MakeRotator` 0.0 0.0 (+ _rot _relativerotation_yaw)) false false))
    (:`Finished`
      (`self.OnFinishRotation`))))

(event `OnFinishRotation`)

(fn `UserConstructionScript`)