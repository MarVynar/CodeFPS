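; BP_Corpse is an environment corpse whose mask, head and limbs can each be present or missing.
; On BeginPlay, boolean flags decide what is removed: the inquisitor mask component is made invisible, and missing body parts are hidden by bone name on the skeletal mesh.
; Hiding happens at the head, calf and lower-arm bones, and only at runtime, as the construction script is empty.
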(event `self.ReceiveBeginPlay`
  (if (not (`self.HasMask`))
    (`SceneComponent.SetVisibility` (`self.SM_Inquisitor_Mask`) false false))
  (if (not (`self.HasHead`))
    (`SkinnedMeshComponent.HideBoneByName` (`self.SkeletalMesh`) "head" "PBO_None"))
  (if (not (`self.HasLLeg`))
    (`SkinnedMeshComponent.HideBoneByName` (`self.SkeletalMesh`) "calf_l" "PBO_None"))
  (if (not (`self.HasRLeg`))
    (`SkinnedMeshComponent.HideBoneByName` (`self.SkeletalMesh`) "calf_r" "PBO_None"))
  (if (not (`self.HasRArm`))
    (`SkinnedMeshComponent.HideBoneByName` (`self.SkeletalMesh`) "lowerarm_r" "PBO_None"))
  (if (not (`self.HasLArm`))
    (`SkinnedMeshComponent.HideBoneByName` (`self.SkeletalMesh`) "lowerarm_l" "PBO_None")))

(fn `UserConstructionScript`)