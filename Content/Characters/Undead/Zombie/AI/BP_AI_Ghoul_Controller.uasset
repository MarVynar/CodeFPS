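; AI controller for ghoul zombies that runs their behavior tree and reacts to sighted enemies.
; On BeginPlay it slows the ghoul's walk and seeds Blackboard AI state from its waypoint and looping settings.
; Pawn sensing records living other-faction characters as known enemies and switches the AI state.
; The following speed-up casts the seen character, not the controlled ghoul, so it only affects sighted ghouls.
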(event `self.ReceiveBeginPlay`
  (bind _blackboard (`self.Blackboard`))
  (bind _blackboard_2 (`self.Blackboard`))
  (bind _blackboard_3 (`self.Blackboard`))
  (bind _asbp_ghoul_base (cast `/Game/Characters/Undead/Zombie/BP_Ghoul_Base` (`self.K2_GetPawn`)))
  (set `CharacterMovementComponent.MaxWalkSpeed` (`CodeFPS_Character_Base.SlowWalkSpeed` _asbp_ghoul_base) (`Character.CharacterMovement` _asbp_ghoul_base))
  (`self.RunBehaviorTree` "/Game/Characters/Undead/Zombie/AI/BT_DEAD_Ghoul.BT_DEAD_Ghoul")
  (set `self.ThisSkeleton` _asbp_ghoul_base)
  (bind _aidecisionparameters (`/Game/Characters/Undead/Zombie/BP_Ghoul_Base.AIDecisionParameters` _asbp_ghoul_base))
  (bind _returnvalue (> (`KismetArrayLibrary.Array_Length` (`AIDecisionParametersComponent.Waypoints` _aidecisionparameters)) 0))
  (if _returnvalue
    (bind _loopwaypoints (`AIDecisionParametersComponent.LoopWaypoints` _aidecisionparameters))
    (`BlackboardComponent.SetValueAsBool` _blackboard "LoopWaypoints" _loopwaypoints)
    (`BlackboardComponent.SetValueAsBool` _blackboard "HasWaypoints" _returnvalue)
    (if _loopwaypoints
      (bind _output_get (set `self.AIState` "NewEnumerator1"))
      (`BlackboardComponent.SetValueAsEnum` _blackboard_2 "AIState" _output_get)
      (`BlackboardComponent.SetValueAsEnum` _blackboard_2 "DefaultAIState" _output_get)
      (else
        (bind _output_get_2 (set `self.AIState` "NewEnumerator4"))
        (`BlackboardComponent.SetValueAsEnum` _blackboard_2 "AIState" _output_get_2)))
    (else
      (bind _output_get_3 (set `self.AIState` "NewEnumerator2"))
      (`BlackboardComponent.SetValueAsEnum` _blackboard_3 "AIState" _output_get_3)
      (`BlackboardComponent.SetValueAsEnum` _blackboard_3 "DefaultAIState" _output_get_3))))

(event `self.PawnSensing.OnSeePawn`
  (params (Pawn :type "Pawn Object Reference"))
  (bind _ascode_fps_character_base (cast `CodeFPS_Character_Base` Pawn))
  (bind _returnvalue (`CodeFPS_Character_Base.AnotherCharacterFromSameFaction` (`self.ThisSkeleton`) _ascode_fps_character_base))
  (if (and (not _returnvalue) (not (`CodeFPS_Character_Base.IsDead` _ascode_fps_character_base)))
    (`KismetArrayLibrary.Array_AddUnique` (`self.KnownEnemies`) _ascode_fps_character_base)
    (if (`|EnumInequality` (`self.AIState`) "NewEnumerator3")
      (bind _output_get (set `self.AIState` "NewEnumerator3"))
      (`BlackboardComponent.SetValueAsEnum` (`self.Blackboard`) "AIState" _output_get)
      (bind _asbp_ghoul_base (cast `/Game/Characters/Undead/Zombie/BP_Ghoul_Base` _ascode_fps_character_base))
      (set `CharacterMovementComponent.MaxWalkSpeed` (`CodeFPS_Character_Base.DefaultWalkSpeed` _asbp_ghoul_base) (`Character.CharacterMovement` _asbp_ghoul_base)))))

(fn `UserConstructionScript`)