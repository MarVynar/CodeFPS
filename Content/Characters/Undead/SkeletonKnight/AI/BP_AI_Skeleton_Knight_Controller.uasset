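; AI controller for the Skeleton Knight that runs its behavior tree and drives the AI state in the Blackboard.
; On BeginPlay it picks the starting state from the pawn's waypoints and loop setting, writing a default state except for non-looping routes.
; PawnSensing adds living characters of other factions to KnownEnemies and switches the state.
; Older player-distance and TargetActor logic remains as unconnected nodes.
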(event `self.ReceiveBeginPlay`
  (bind _blackboard (`self.Blackboard`))
  (bind _blackboard_2 (`self.Blackboard`))
  (bind _blackboard_3 (`self.Blackboard`))
  (bind _asbp_skeleton_knight_base (cast `/Game/Characters/Undead/SkeletonKnight/BP_SkeletonKnight_Base` (`self.K2_GetPawn`)))
  (`self.RunBehaviorTree` "/Game/Characters/Undead/SkeletonKnight/AI/BT_DEAD_Skeleton_Warrior.BT_DEAD_Skeleton_Warrior")
  (set `self.ThisSkeleton` _asbp_skeleton_knight_base)
  (bind _aidecisionparameters (`/Game/Characters/Undead/SkeletonKnight/BP_SkeletonKnight_Base.AIDecisionParameters` _asbp_skeleton_knight_base))
  (bind _returnvalue (> (`KismetArrayLibrary.Array_Length` (`AIDecisionParametersComponent.Waypoints` _aidecisionparameters)) 0))
  (if _returnvalue
    (bind _loopwaypoints (`AIDecisionParametersComponent.LoopWaypoints` _aidecisionparameters))
    (`BlackboardComponent.SetValueAsBool` _blackboard "LoopWaypoints" _loopwaypoints)
    (`BlackboardComponent.SetValueAsBool` _blackboard "HasWaypoints" _returnvalue)
    (if _loopwaypoints
      (bind _output_get (set `self.AIState` "NewEnumerator1"))
      (`BlackboardComponent.SetValueAsEnum` _blackboard_2 "AIState" _output_get)
      (`BlackboardComponent.SetValueAsEnum` _blackboard_2 "DefaultAIState" _output_get)
      (else
        (bind _output_get_2 (set `self.AIState` "NewEnumerator4"))
        (`BlackboardComponent.SetValueAsEnum` _blackboard_2 "AIState" _output_get_2)))
    (else
      (bind _output_get_3 (set `self.AIState` "NewEnumerator2"))
      (`BlackboardComponent.SetValueAsEnum` _blackboard_3 "AIState" _output_get_3)
      (`BlackboardComponent.SetValueAsEnum` _blackboard_3 "DefaultAIState" _output_get_3))))

(event `self.PawnSensing.OnSeePawn`
  (params (Pawn :type "Pawn Object Reference"))
  (bind _ascode_fps_character_base (cast `CodeFPS_Character_Base` Pawn))
  (bind _returnvalue (`CodeFPS_Character_Base.AnotherCharacterFromSameFaction` (`self.ThisSkeleton`) _ascode_fps_character_base))
  (if (and (not _returnvalue) (not (`CodeFPS_Character_Base.IsDead` _ascode_fps_character_base)))
    (`KismetArrayLibrary.Array_AddUnique` (`self.KnownEnemies`) _ascode_fps_character_base)
    (bind _output_get (set `self.AIState` "NewEnumerator3"))
    (`BlackboardComponent.SetValueAsEnum` (`self.Blackboard`) "AIState" _output_get)))

(fn `UserConstructionScript`)