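; Base Blueprint for a Skeleton Knight undead character that can evade or block incoming projectiles.
; When a projectile enters its interaction collision while alive, random rolls pick a dash, the child-actor block ability, or no reaction.
; Dash jumps and timeline-lerps the actor, without sweep, to a trace end along the mesh's positive or negative forward axis, ignoring hits.
; A second timeline blends walk speed on state updates, then signals completion.
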(event `self.ReceiveBeginPlay`
  (`parent.ReceiveBeginPlay`))

(event `self.OnInteractionCollisionBegin`
  (params (overlappedComponent :type "PrimitiveComponent Object Reference") (otherActor :type "Actor Object Reference") (otherComp :type "PrimitiveComponent Object Reference") (otherBodyIndex :type Integer) (fromSweep :type Boolean) (sweepResult :type "HitResult Structure (by ref)"))
  (bind _returnvalue (`KismetMathLibrary.RandomIntegerInRange` 0 100))
  (cast `CodeFPS_Proj_Base` otherActor)
  (if (`self.IsDead`)
    _
    (elif (<= _returnvalue (`self.DashChance`))
      (`self.Dash`)
      (elif (<= _returnvalue (+ (`self.DashChance`) (`self.BlockChance`)))
        (bind _ascode_fps_ability_base (cast `CodeFPS_Ability_Base` (`ChildActorComponent.ChildActor` (`self.Ability_Skeleton_Block`))))
        (`self.UseAbility` _ascode_fps_ability_base)
        (`KismetSystemLibrary.PrintString` "BLOCK" true true (struct :`G` 1.0 :`B` 0.159328 :`A` 1.0) 9.0)))))

(event `self.Dash`
  (bind _returnvalue (`SceneComponent.K2_GetComponentLocation` (`self.CapsuleComponent`)))
  (`self.Jump`)
  (if (`KismetMathLibrary.RandomBool`)
    (bind _outhit (`KismetSystemLibrary.LineTraceSingle` _returnvalue (+ (* (`SceneComponent.GetForwardVector` (`self.Mesh`)) (`self.DashDistance`)) _returnvalue) "TraceTypeQuery1"))
    (set `self.DashDestination` (`.TraceEnd` (`GameplayStatics.BreakHitResult` _outhit)))
    (bind (_direction _alpha) (`Timeline|Timeline_0` :!via `PlayFromStart` :!label _label)
      (:`Update`
        (`self.K2_SetActorLocation` (`KismetMathLibrary.VLerp` (`self.K2_GetActorLocation`) (`self.DashDestination`) _alpha))))
    (else
      (bind _outhit_2 (`KismetSystemLibrary.LineTraceSingle` _returnvalue (+ _returnvalue (* (* (`SceneComponent.GetForwardVector` (`self.Mesh`)) (`self.DashDistance`)) -1.0)) "TraceTypeQuery1"))
      (set `self.DashDestination` (`.TraceEnd` (`GameplayStatics.BreakHitResult` _outhit_2)))
      (goto _label :!via `PlayFromStart`))))

(event `self.ReceiveAnyDamage`
  (params (Damage :type "Float (single-precision)") (DamageType :type "DamageType Object Reference") (InstigatedBy :type "Controller Object Reference") (DamageCauser :type "Actor Object Reference"))
  (`parent.ReceiveAnyDamage` Damage DamageType InstigatedBy DamageCauser))

(event `SpeedStateUpdate`
  (params (Initial :type "Float (double-precision)") (Final :type "Float (double-precision)"))
  (bind (_direction _speedupd) (`Timeline|SpeedUpdateTimeline` :!via `PlayFromStart`)
    (:`Update`
      (set `CharacterMovementComponent.MaxWalkSpeed` (`KismetMathLibrary.Lerp` Initial Final _speedupd) (`self.CharacterMovement`)))
    (:`Finished`
      (`self.DSpeedUpdated`))))

(fn `UserConstructionScript`)